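; Battle royale zone actor that represents the safe zone in the world and renders it into a mask render target.
; Size and location update events scale the actor in X/Y and move it.
; Each Tick clears the render target and draws a circle mask texture positioned and sized from normalized safe zone coordinates.
; GetNextZoneStageLocation offsets the current center in a random yaw direction, by a random distance bounded by the stage size difference.
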(event EventTick
  (params (DeltaSeconds :type Float%20%28single-precision%29))
  (bind _returnvalue (Class|BRZoneActor|GetSafeZoneCoords))
  (bind _safeareasrendertarget (Variables|Default|GetSafeAreasRenderTarget))
  (bind (_x _y _z) (Math|Vector|BreakVector _returnvalue))
  (Rendering|ClearRenderTarget2D _safeareasrendertarget)
  (bind (_canvas _size _context) (Rendering|BeginDrawCanvastoRenderTarget _safeareasrendertarget))
  (Canvas|DrawTexture :self _canvas :RenderTexture "/Game/GameModes/BR/UI/CircleMaskTexture.CircleMaskTexture" :ScreenPosition (- (* _size (Math|Vector2D|MakeVector2D _x _y)) (/ (* _size (Math|Vector2D|MakeVector2D _z _z)) 2.0)) :ScreenSize (* _size (Math|Vector2D|MakeVector2D _z _z)) :CoordinateSize "(X=1.000000,Y=1.000000)" :PivotPoint "(X=0.500000,Y=0.500000)")
  (Rendering|EndDrawCanvastoRenderTarget _context))

(event EventZoneSizeUpdate
  (params (val :type Float%20%28single-precision%29))
  (Transformation|SetActorScale3D (Math|Vector|MakeVector val val (.Z (Math|Vector|BreakVector (Transformation|GetActorScale3D))))))

(event EventZoneLocationUpdate
  (params (val :type Vector :default "0, 0, 0"))
  (Transformation|SetActorLocation val false false))

(fn ConstructionScript)

(fn GetNextZoneStageLocation
  (params (CurrentLocation :type Vector :default "0, 0, 0") (ZoneStageSizeDiff :type Float%20%28single-precision%29))
  (return (+ CurrentLocation (Math|Vector|RotateVector (* (Math|Vector|MakeVector (Math|Random|RandomFloatinRange 0.0 ZoneStageSizeDiff) 0.0 0.0) 50) (Math|Rotator|MakeRotator 0.0 0.0 (Math|Random|RandomFloatinRange -1.8e+02 1.8e+02))))))