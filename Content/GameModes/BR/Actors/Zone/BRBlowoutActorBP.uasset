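; BRBlowoutActorBP is the battle royale blowout zone actor that paints a mask of the current safe areas into a render target.
; Every tick it clears SafeAreasRenderTarget to a grayscale value from GetOutsideSafetyLevel, then opens a canvas on it.
; It stamps a circle mask texture for each entry from GetSafeZonesCoords, using XY as normalized center and Z as size relative to the target.
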(event EventTick
  (params (DeltaSeconds :type Float%20%28single-precision%29))
  (bind _returnvalue (Class|BRBlowoutActor|GetOutsideSafetyLevel))
  (bind _safeareasrendertarget (Variables|Default|GetSafeAreasRenderTarget))
  (Rendering|ClearRenderTarget2D _safeareasrendertarget (Math|Color|MakeColor _returnvalue _returnvalue _returnvalue))
  (bind (_canvas _size _context) (Rendering|BeginDrawCanvastoRenderTarget _safeareasrendertarget))
  (for _array_element (Class|BRBlowoutActor|GetSafeZonesCoords)
    (Canvas|DrawTexture :self _canvas :RenderTexture "/Game/GameModes/BR/UI/CircleMaskTexture.CircleMaskTexture" :ScreenPosition (- (* _size (Math|Vector2D|MakeVector2D (.X (Math|Vector|BreakVector _array_element)) (.Y (Math|Vector|BreakVector _array_element)))) (/ (* _size (Math|Vector2D|MakeVector2D (.Z (Math|Vector|BreakVector _array_element)) (.Z (Math|Vector|BreakVector _array_element)))) 2.0)) :ScreenSize (* _size (Math|Vector2D|MakeVector2D (.Z (Math|Vector|BreakVector _array_element)) (.Z (Math|Vector|BreakVector _array_element)))) :CoordinateSize "(X=1.000000,Y=1.000000)" :PivotPoint "(X=0.500000,Y=0.500000)"))
  (Rendering|EndDrawCanvastoRenderTarget _context))

(fn ConstructionScript)