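; FirearmWeaponItemBP is the Blueprint for a firearm weapon item that fires projectiles.
; Its CreateProjectile event always spawns a CubitUniProjectile at the given transform, passing bullet speed, size, attack ID, itself and the player character as instigator.
; Each projectile gets a life span from the weapon's bullet setting.
; A GetSpawnTransformOffset function returns a fixed offset, slightly raised and rotated a quarter turn.
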(event EventCreateProjectile
  (params (Transform :type Transform) (attackId :type Integer))
  (bind _returnvalue (Game|SpawnActorfromClass "/Game/BallisticsVFX/FXSpawnerBlueprints/Projectiles/CubitUniProjectile.CubitUniProjectile_C" Transform "AlwaysSpawn" (Components|GetOwner) (Math|Conversions|ToFloat(Integer) (Variables|Default|GetBulletSpeed)) true true false (Variables|Default|GetProjectileSize) 0 "NewEnumerator0" self attackId (Variables|Default|GetPlayerCharacter)))
  (Actor|SetLifeSpan _returnvalue (Variables|Default|GetBulletLifeSpanSec)))

(fn ConstructionScript)

(fn GetSpawnTransformOffset
  (return (Math|Transform|MakeTransform "0, 0,3.000000" "90.000000, 0, 0")))