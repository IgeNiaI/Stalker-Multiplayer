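; Player character Blueprint whose functions classify a skeletal mesh bone as a body part: Head, Arm, Leg or Body.
; BoneToBodyPart tests the bone against the head, left and right clavicle, and left and right thigh roots, falling back to Body.
; IsBoneChildOrEqual supplies each test, matching the root bone itself or any bone below it in the Mesh hierarchy.
; The construction script is empty.
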(fn ConstructionScript)

(fn BonetoBodyPart
  (params (BoneName :type Name :default "None"))
  (if (CallFunction|IsBoneChildorEqual BoneName "bip01_head")
    (return "Head")
    (elif (or (CallFunction|IsBoneChildorEqual BoneName "bip01_l_clavicle") (CallFunction|IsBoneChildorEqual BoneName "bip01_r_clavicle"))
      (return "Arm")
      (elif (or (CallFunction|IsBoneChildorEqual BoneName "bip01_l_thigh") (CallFunction|IsBoneChildorEqual BoneName "bip01_r_thigh"))
        (return "Leg")
        (else
          (return "Body"))))))

(fn IsBoneChildorEqual
  (params (BoneName :type Name) (ParentBoneName :type Name))
  (return (or (Utilities|Name|Equal(Name) BoneName ParentBoneName) (Class|SkinnedMeshComponent|BoneIsChildOf (Variables|Character|GetMesh) BoneName ParentBoneName))))