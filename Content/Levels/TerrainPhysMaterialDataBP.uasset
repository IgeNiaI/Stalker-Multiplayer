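; Level actor for terrain physical material data that turns the terrain mask texture into a render target.
; On BeginPlay, only on the remote (non-authority) side, it creates a render target matching the mask's size.
; It draws the mask across the whole canvas with opaque blending, then hands the result to SetTerrainMaskRenderTarget.
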(event EventBeginPlay
  (bind _terrainmask (Variables|Default|GetTerrainMask))
  (Networking|SwitchHasAuthority
    (:Remote
      (bind _returnvalue (Rendering|CreateRenderTarget2D (Class|Texture2D|BlueprintGetSizeX _terrainmask) (Class|Texture2D|BlueprintGetSizeY _terrainmask) "RTF_RGBA16f"))
      (bind _output_get (Variables|Default|SetRenderTarget _returnvalue))
      (bind (_canvas _size _context) (Rendering|BeginDrawCanvastoRenderTarget _output_get))
      (Canvas|DrawTexture :self _canvas :RenderTexture (Variables|Default|GetTerrainMask) :ScreenSize _size :CoordinateSize "(X=1.000000,Y=1.000000)" :BlendMode "BLEND_Opaque" :PivotPoint "(X=0.500000,Y=0.500000)")
      (Rendering|EndDrawCanvastoRenderTarget _context)
      (Class|TerrainPhysMaterialData|SetTerrainMaskRenderTarget (Variables|Default|GetRenderTarget)))))

(fn ConstructionScript)